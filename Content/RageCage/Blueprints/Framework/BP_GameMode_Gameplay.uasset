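; Gameplay game mode that spawns tracker bots and awards score for kills.
; SpawnNewBot runs an EQS query picking randomly from the best 25% of locations, then spawns BP_TrackerBot at the result with a debug sphere.
; An actor-killed delegate bound on BeginPlay adds points to the killer's SPlayerState when a non-player pawn dies, printing the score.
; PostLogin only casts the new player controller, with no further logic.
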(event Custom|OnActorKilled_Event_0
  (params (VictimActor :type Actor%20Object%20Reference) (KillerActor :type Actor%20Object%20Reference) (KillerController :type Controller%20Object%20Reference))
  (bind _aspawn (Utilities|Casting|CastToPawn VictimActor))
  (if (not (Pawn|IsPlayerControlled _aspawn))
    (Utilities|IsValid KillerController
      (:Is%20Valid
        (bind _assplayer_state (Utilities|Casting|CastToSPlayerState (Variables|/Script/Engine.Pawn|GetPlayerState (Pawn|GetControlledPawn KillerController))))
        (Class|SPlayerState|AddScore _assplayer_state 2e+01)
        (Development|PrintString (Utilities|String|ToString(Float) (Variables|/Script/Engine.PlayerState|GetScore _assplayer_state)) true true "(R=1.000000,G=0.099356,B=0.039631,A=1.000000)")))))

(event Custom|OnQueryFinishedEvent_Event_0
  (params (QueryInstance :type Env%20Query%20Instance%20Blueprint%20Wrapper%20Object%20Reference) (QueryStatus :type EEnvQueryStatus%20Enum :default "Processing"))
  (switch Utilities|FlowControl|Switch|SwitchonEEnvQueryStatus QueryStatus
    (:Success
      (for _array_element (Class|EnvQueryInstanceBlueprintWrapper|GetResultsasLocations QueryInstance)
        (Rendering|Debug|DrawDebugSphere _array_element 5e+01 12 "(R=1.000000,G=0.922361,B=0.000000,A=1.000000)" 2.0 2.0)
        (Game|SpawnActorfromClass "/Game/RageCage/Blueprints/Actors/TrackerBot/BP_TrackerBot.BP_TrackerBot_C" (Math|Transform|MakeTransform _array_element) "AdjustIfPossibleButDontSpawnIfColliding" 0 0)))))

(event EventBeginPlay
  (EventDispatchers|AssignOnActorKilled (delegate Custom|OnActorKilled_Event_0)))

(event EventSpawnNewBot
  (bind _returnvalue (AI|EQS|RunEQSQuery "/Game/RageCage/Blueprints/Framework/EQS_FindSpawnLocation.EQS_FindSpawnLocation" self "RandomBest25Pct"))
  (EventDispatchers|AssignOnQueryFinishedEvent _returnvalue (delegate Custom|OnQueryFinishedEvent_Event_0)))

(event EventPostLogin
  (params (NewPlayer :type Player%20Controller%20Object%20Reference))
  (Utilities|Casting|CastToBP_PlayerController NewPlayer))

(fn ConstructionScript)