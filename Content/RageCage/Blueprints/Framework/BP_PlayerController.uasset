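; Player controller that sets up the player's HUD and handles the pause menu.
; BeginPlay adds the health indicator and crosshair widgets to the viewport.
; The Pause action toggles a pause flag, adding or removing the menu and switching between UI-only and game-only input.
; It never calls SetGamePaused, and it hides the cursor on unpause without showing it on pause.
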(event EventBeginPlay
  (Utilities|FlowControl|Sequence
    (:then_0
      (bind _returnvalue (UserInterface|CreateWidget "/Game/RageCage/UI/WBP_HealthIndicator.WBP_HealthIndicator_C"))
      (UserInterface|Viewport|AddtoViewport _returnvalue 0))
    (:then_1
      (bind _returnvalue_2 (UserInterface|CreateWidget "/Game/RageCage/UI/WBP_Crosshair.WBP_Crosshair_C"))
      (UserInterface|Viewport|AddtoViewport _returnvalue_2 0))))

(event Input|ActionEvents|InputActionPause
  (params (Key :type Key%20Structure))
  ;[1 1 1] Pause / Unpause
  (:Pressed
    (if (Variables|Default|GetIsGamePaused?)
      (Variables|Default|SetIsGamePaused? false)
      (Widget|RemovefromParent (stale _returnvalue))
      (Variables|Default|SetbShowMouseCursor false)
      (Input|SetInputModeGameOnly self)
      (else
        (Variables|Default|SetIsGamePaused? true)
        (bind _returnvalue (UserInterface|CreateWidget "/Game/RageCage/UI/WBP_PauseMenu.WBP_PauseMenu_C"))
        (UserInterface|Viewport|AddtoViewport _returnvalue 0)
        (Input|SetInputModeUIOnly self 0 "DoNotLock")))))

(fn ConstructionScript)