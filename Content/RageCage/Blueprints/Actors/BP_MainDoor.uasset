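; BP_MainDoor is a door that the player opens with the Interact input and that moves again when the player enters a separate close trigger.
; A box overlap with BP_Player shows a text prompt and enables interaction while the door is unopened.
; Interacting plays the DoorOpen timeline to move the door along relative Z with sweep.
; DoorCloseCollision prints a debug string, clears the opened flag and plays a second timeline on the same axis.
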(event OnComponentBeginOverlap(Box)
  (params (OverlappedComponent :type Primitive%20Component%20Object%20Reference) (OtherActor :type Actor%20Object%20Reference) (OtherComp :type Primitive%20Component%20Object%20Reference) (OtherBodyIndex :type Integer) (bFromSweep :type Boolean) (SweepResult :type Hit%20Result%20Structure%20%28by%20ref%29))
  (Utilities|Casting|CastToBP_Player OtherActor)
  (if (not (Variables|Default|GetbHasBeenOpened))
    (Rendering|SetVisibility (Variables|Default|GetTextRender) true false)
    (Variables|Default|SetbCanOpenDoor true)))

(event OnComponentEndOverlap(Box)
  (params (OverlappedComponent :type Primitive%20Component%20Object%20Reference) (OtherActor :type Actor%20Object%20Reference) (OtherComp :type Primitive%20Component%20Object%20Reference) (OtherBodyIndex :type Integer))
  (Utilities|Casting|CastToBP_Player OtherActor)
  (Rendering|SetVisibility (Variables|Default|GetTextRender) false false)
  (Variables|Default|SetbCanOpenDoor false))

(event OnComponentBeginOverlap(DoorCloseCollision)
  (params (OverlappedComponent :type Primitive%20Component%20Object%20Reference) (OtherActor :type Actor%20Object%20Reference) (OtherComp :type Primitive%20Component%20Object%20Reference) (OtherBodyIndex :type Integer) (bFromSweep :type Boolean) (SweepResult :type Hit%20Result%20Structure%20%28by%20ref%29))
  (Development|PrintString "Hello")
  (Utilities|Casting|CastToBP_Player OtherActor)
  (Rendering|SetVisibility (Variables|Default|GetTextRender) false false)
  (Variables|Default|SetbHasBeenOpened false)
  (bind _openspeed (Timeline|Timeline_0 Play)
    (:Update
      (Transformation|SetRelativeLocation (Variables|Default|GetDoor) (Math|Vector|MakeVector 0.0 0.0 _openspeed) true false))))

(event EventBeginPlay
  (Input|EnableInput (Game|GetPlayerController 0)))

(event Input|ActionEvents|InputActionInteract
  (params (Key :type Key%20Structure))
  (:Pressed
    (if (Variables|Default|GetbCanOpenDoor)
      (Rendering|SetVisibility (Variables|Default|GetTextRender) false false)
      (Variables|Default|SetbHasBeenOpened true)
      (bind _openspeed (Timeline|DoorOpen Play)
        (:Update
          (Transformation|SetRelativeLocation (Variables|Default|GetDoor) (Math|Vector|MakeVector 0.0 0.0 _openspeed) true false))))))

(fn ConstructionScript)