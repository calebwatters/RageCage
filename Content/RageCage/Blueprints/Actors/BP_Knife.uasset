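; BP_Knife is a melee knife actor that damages TPSCharacters its blade collision touches, ignoring its own instigator.
; An overlap on DamageBlade applies fixed damage with the knife as causer, then plays an impact sound and a blood spurt at the knife's location.
; A DoOnce gate, reset after a short delay, acts as a hit cooldown shared across all targets.
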(event OnComponentBeginOverlap(DamageBlade)
  (params (OverlappedComponent :type Primitive%20Component%20Object%20Reference) (OtherActor :type Actor%20Object%20Reference) (OtherComp :type Primitive%20Component%20Object%20Reference) (OtherBodyIndex :type Integer) (bFromSweep :type Boolean) (SweepResult :type Hit%20Result%20Structure%20%28by%20ref%29))
  (bind _returnvalue (Transformation|GetActorLocation))
  (bind _astpscharacter (Utilities|Casting|CastToTPSCharacter OtherActor))
  (if (not (== (Game|GetInstigator) OtherActor))
    (Utilities|FlowControl|DoOnce false :!label _label
      (:Completed
        (Game|Damage|ApplyDamage _astpscharacter 3e+01 0 self)
        (Audio|PlaySoundatLocation "/Game/MilitaryWeapDark/Sound/Knife/Knife_ImpactBody_Cue.Knife_ImpactBody_Cue" _returnvalue)
        (Effects|SpawnEmitteratLocation "/Game/FXVillesBloodVFXPack/Particles/PS_Blood_Spurt_01.PS_Blood_Spurt_01" _returnvalue "90.000000,0.000000,90.000000" "0.500000,0.500000,0.500000")
        (Utilities|FlowControl|Delay 0.8)
        (goto _label Reset)))))

(fn ConstructionScript)